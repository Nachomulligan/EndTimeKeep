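; Enemy projectile, filed under the boss enemy, that flies at a target and damages the first-person player character.
; On BeginPlay with a valid Target, it aims once at the target's location at fixed speed, without homing, and self-destructs after a timeout.
; Box overlap casts the sweep result's hit actor to the player character, then spawns an emitter there, applies Damage and destroys the projectile.
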(event OnComponentBeginOverlap(Box)
  (params (OverlappedComponent :type Primitive%20Component%20Object%20Reference) (OtherActor :type Actor%20Object%20Reference) (OtherComp :type Primitive%20Component%20Object%20Reference) (OtherBodyIndex :type Integer) (bFromSweep :type Boolean) (SweepResult :type Hit%20Result%20Structure%20%28by%20ref%29))
  (bind _hitactor (Collision|BreakHitResult SweepResult))
  (bind _asbp_first_person_character (Utilities|Casting|CastToBP_FirstPersonCharacter _hitactor))
  (if (== _asbp_first_person_character _hitactor)
    (Effects|SpawnEmitteratLocation 0 (Transformation|GetActorLocation _hitactor))
    (Game|Damage|ApplyDamage _hitactor (Variables|Default|GetDamage) 0 0)
    (Actor|DestroyActor)))

(event Custom|Aim%20At%20Target
  (bind _output_get (Variables|/Script/Engine.MovementComponent|SetVelocity (Variables|Default|GetProjectileMovement) (* (Math|Vector|GetUnitDirection(Vector) (Transformation|GetActorLocation) (Transformation|GetActorLocation (Variables|Default|GetTarget))) 8e+02)))
  (Transformation|SetActorRotation (Math|Conversions|RotationFromXVector _output_get)))

(event EventBeginPlay
  (Variables|Default|GetTarget
    (:then
      (CallFunction|AimatTarget)
      (Utilities|FlowControl|Delay 1e+01)
      (Actor|DestroyActor))
    (:else)))

(fn ConstructionScript)