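; Boss enemy that spawns ever-growing waves of regular enemies and shows the victory screen when killed.
; A looping delay drives waves, staggering spawns at random reachable navmesh points around the boss.
; Damage depletes its health until it explodes, while Attack fires a projectile targeting the player.
; PawnSensing sets the seesPlayer blackboard key for pawns with an allied health component, clearing it when that health depletes.
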(event OnSeePawn(PawnSensing)
  (params (Pawn :type Pawn%20Object%20Reference))
  (bind _returnvalue (Actor|GetComponentbyClass Pawn "/Game/Owned/Component/AC_HealthAllies.AC_HealthAllies_C"))
  ;[1 1 1] PawnSensing with Target Death
  (if true
    (Actor|GetAllActorswithTag "Damageable")
    (Utilities|IsValid _returnvalue
      (:Is%20Valid
        (EventDispatchers|BindEventtoOnHealthDepleted _returnvalue (delegate Custom|OnTargetDeath))
        (AI|Components|Blackboard|SetValueasBool (AI|GetBlackboard (AI|GetAIController self)) (Utilities|Name|MakeLiteralName "seesPlayer") true)
        (Development|PrintString "ESTÁ SETEADO")))))

(event Custom|Spawn
  (bind _waveamount (Variables|Default|GetWaveAmount))
  (Utilities|FlowControl|Sequence
    (:then_0
      (bind _output_get (Variables|Default|SetEnemiesSpawned _waveamount))
      (if (> _output_get 0) :!label _label
        (Utilities|FlowControl|Delay 0.5)
        (Game|SpawnActorfromClass "/Game/Owned/Enemies/Regular_Enemy/BP_RegularEnemy.BP_RegularEnemy_C" (Math|Transform|MakeTransform (.RandomLocation (AI|Navigation|GetRandomReachablePointinRadius (Transformation|GetActorLocation) 1e+03 0 0)) "0, 0, 0" "1.000000,1.000000,1.000000") "Undefined" "MultiplyWithRoot" 0 0)
        (Variables|Default|SetOtherWaves (Variables|Default|GetCooldon%20Waves))
        (Math|Integer|DecrementInt (Variables|Default|GetEnemiesSpawned)
          (:%20%20
            (goto _label)))))
    (:then_1
      (Variables|Default|SetEnemiesAlive _waveamount))))

(event Custom|Attack
  (bind _asbp_first_person_character (Utilities|Casting|CastToBP_FirstPersonCharacter (Game|GetPlayerCharacter 0)))
  (Game|SpawnActorfromClass "/Game/Owned/Enemies/Boss_Enemy/BP_EnemyProjectile.BP_EnemyProjectile_C" (Transformation|GetWorldTransform (Variables|Default|GetScene)) "Undefined" "MultiplyWithRoot" 0 _asbp_first_person_character 0)
  (Default|CallEndAttack))

(event Custom|Death
  (Effects|SpawnEmitteratLocation "/Game/StarterContent/Particles/P_Explosion.P_Explosion" (Transformation|GetWorldLocation (Variables|Default|GetSkeletalMesh)) "0, 0, 0" "2.000000,2.000000,2.000000")
  (Actor|DestroyActor)
  (bind _returnvalue (UserInterface|CreateWidget "/Game/Owned/HUD/WB_Victory.WB_Victory_C"))
  (bind _output_get (Variables|Default|SetVictoryScreen _returnvalue))
  (UserInterface|Viewport|AddtoViewport _output_get 0))

(event Custom|Increase%20Wave%20Amount
  (Variables|Default|SetWaveAmount (+ (Variables|Default|GetWaveAmount) (Variables|Default|GetExtra%20Enemies))))

(event Custom|OnTargetDeath
  ;[1 1 1] PawnSensing with Target Death
  (Development|PrintText "Target is dead!")
  (CallFunction|NotSensing))

(event Custom|NotSensing
  ;[1 1 1] NotSensing Event
  (AI|Components|Blackboard|SetValueasBool (AI|GetBlackboard (AI|GetAIController self)) (Utilities|Name|MakeLiteralName "seesPlayer") false))

(event Game|Damage|EventAnyDamage
  (params (Damage :type Float%20%28single-precision%29) (DamageType :type Damage%20Type%20Object%20Reference) (InstigatedBy :type Controller%20Object%20Reference) (DamageCauser :type Actor%20Object%20Reference))
  ;[1 1 1] Enemy Health
  (if (> (Variables|Default|GetCurrentHealth) 0.0)
    (bind _output_get (Variables|Default|SetCurrentHealth (- (Variables|Default|GetCurrentHealth) Damage)))
    (if (<= _output_get 0.0)
      (CallFunction|Death))))

(event EventBeginPlay
  (Utilities|FlowControl|Delay (Variables|Default|GetFirstWave))
  (Variables|Default|SetIsWaveStarting true :!label _label)
  (if true
    (CallFunction|Spawn)
    (CallFunction|IncreaseWaveAmount)
    (Utilities|FlowControl|Delay (Variables|Default|GetOtherWaves))
    (goto _label)))

(fn ConstructionScript)