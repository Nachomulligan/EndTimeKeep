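; Regular enemy that tracks its health on a camera-facing bar and, on death, explodes, awards resources to the player and destroys itself.
; Blackboard flags track random movement and sight, with PawnSensing flagging seen pawns that have AC_HealthAllies and clearing the flag when their health depletes.
; AttackEnemy damages every forward multi-sphere-trace hit.
; CustomEvent is a single-hit variant with debug drawing, and the projectile Attack is disabled.
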(event OnSeePawn(PawnSensing)
  (params (Pawn :type Pawn%20Object%20Reference))
  (bind _returnvalue (Actor|GetComponentbyClass Pawn "/Game/Owned/Component/AC_HealthAllies.AC_HealthAllies_C"))
  ;[1 1 1] PawnSensing with Target Death
  (if true
    (CallFunction|FinishedMovingtoRandomPoint)
    (Actor|GetAllActorswithTag "Damageable")
    (Utilities|IsValid _returnvalue
      (:Is%20Valid
        (EventDispatchers|BindEventtoOnHealthDepleted _returnvalue (delegate Custom|OnTargetDeath))
        (AI|Components|Blackboard|SetValueasBool (AI|GetBlackboard (AI|GetAIController self)) (Utilities|Name|MakeLiteralName "isSeeingPlayer") true)))))

(event Custom|AttackEnemy
  (bind _returnvalue (Transformation|GetActorLocation))
  ;[1 1 1] Enemy Attack With Sphere Trace
  (bind (_outhits _returnvalue_2) (Collision|MultiSphereTraceByChannel _returnvalue (+ (* (Transformation|GetActorForwardVector self) 2.5e+02) _returnvalue) 2e+02 "TraceTypeQuery4" false 0 "None"))
  (if _returnvalue_2
    (for _array_element _outhits
      (Game|Damage|ApplyDamage (.HitActor (Collision|BreakHitResult _array_element)) (Variables|Default|GetBase%20Damage) 0 0))
    (Effects|SpawnEmitteratLocation 0 (Transformation|GetWorldLocation (Variables|Character|GetMesh)))
    (Development|PrintString "ataccking")))

(event Custom|Attack
  (Game|SpawnActorfromClass "/Game/Owned/Enemies/Regular_Enemy/BP_EnemyProjectile.BP_EnemyProjectile_C" (Transformation|GetWorldTransform (Variables|Default|GetScene)) "Undefined" "MultiplyWithRoot" 0 (Variables|Default|GetAs%20BP%20First%20Person%20Character) 0)
  (Default|CallEndAttack))

(event Custom|Death
  ;[1 1 1] EnemyDeath
  (Effects|SpawnEmitteratLocation "/Game/StarterContent/Particles/P_Explosion.P_Explosion" (Transformation|GetWorldLocation (Variables|Character|GetMesh)) "0, 0, 0" "2.000000,2.000000,2.000000")
  (bind _asbp_first_person_character (Utilities|Casting|CastToBP_FirstPersonCharacter (Game|GetPlayerCharacter 0)))
  (Default|EarnResources _asbp_first_person_character (Variables|Default|GetResources%20Earned))
  (Actor|DestroyActor))

(event Custom|CustomEvent
  (bind _returnvalue (Transformation|GetActorLocation))
  (bind _self self)
  (bind _returnvalue_2 (Transformation|GetActorForwardVector _self))
  (bind _returnvalue_3 (* _returnvalue_2 2.5e+02))
  (bind _returnvalue_4 (+ _returnvalue_3 _returnvalue))
  ;[1 1 1] Enemy Attack With Sphere Trace
  (Collision|MultiSphereTraceByChannel _returnvalue _returnvalue_4 2e+02 "TraceTypeQuery1" false 0 "None")
  (bind (_outhit _returnvalue_5) (Collision|SphereTraceForObjects _returnvalue _returnvalue_4 2e+02 (Utilities|Array|MakeArray "ObjectTypeQuery3") false 0 "ForDuration"))
  (if _returnvalue_5
    (Game|Damage|ApplyDamage (.HitActor (Collision|BreakHitResult _outhit)) (Variables|Default|GetBase%20Damage) 0 0)
    (Effects|SpawnEmitteratLocation 0 (Transformation|GetWorldLocation (Variables|Character|GetMesh)))
    (Development|PrintString "ataccking")))

(event Custom|OnTargetDeath
  ;[1 1 1] PawnSensing with Target Death
  (Development|PrintText "Target is dead!")
  (CallFunction|NotSensing))

(event Custom|NotSensing
  ;[1 1 1] NotSensing Event
  (AI|Components|Blackboard|SetValueasBool (AI|GetBlackboard (AI|GetAIController self)) (Utilities|Name|MakeLiteralName "isSeeingPlayer") false))

(event Custom|FinishedMovingToRandomPoint
  (AI|Components|Blackboard|SetValueasBool (AI|GetBlackboard (AI|GetAIController self)) (Utilities|Name|MakeLiteralName "isMovingToRandomPoint") false))

(event Game|Damage|EventAnyDamage
  (params (Damage :type Float%20%28single-precision%29) (DamageType :type Damage%20Type%20Object%20Reference) (InstigatedBy :type Controller%20Object%20Reference) (DamageCauser :type Actor%20Object%20Reference))
  ;[1 1 1] Enemy Health
  (if (> (Variables|Default|GetCurrentHealth) 0.0)
    (bind _output_get (Variables|Default|SetCurrentHealth (- (Variables|Default|GetCurrentHealth) Damage)))
    (if (<= _output_get 0.0)
      (CallFunction|Death))))

(event EventTick
  (params (DeltaSeconds :type Float%20%28single-precision%29))
  (bind _healthbar (Variables|Default|GetHealthBar))
  ;[1 1 1] Health Bar Config
  (Progress|SetPercent (Variables|/Game/Owned/HUD/WB_HealthBar.WB_HealthBar_C|GetHealthBar (Variables|Default|GetAs%20WB%20Health%20Bar)) (/ (Variables|Default|GetCurrentHealth) (Variables|Default|GetMaxHealth)))
  (Transformation|SetWorldRotation _healthbar (Math|Rotator|FindLookatRotation (Transformation|GetWorldLocation _healthbar) (Transformation|GetWorldLocation (Variables|/Script/Engine.Actor|GetRootComponent (Game|GetPlayerCameraManager 0)))) false false))

(event EventBeginPlay
  ;[1 1 1] Health Bar Config
  (bind _aswb_health_bar (Utilities|Casting|CastToWB_HealthBar (UserInterface|GetUserWidgetObject (Variables|Default|GetHealthBar))))
  (Variables|Default|SetAs%20WB%20Health%20Bar _aswb_health_bar)
  (AI|Components|Blackboard|SetValueasBool (AI|GetBlackboard (AI|GetAIController self)) (Utilities|Name|MakeLiteralName "isMovingToRandomPoint") true))

(fn ConstructionScript)