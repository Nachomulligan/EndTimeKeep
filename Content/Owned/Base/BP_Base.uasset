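; BP_Base is a base actor with health that regular enemies damage by hitting it, ending in a defeat screen.
; A blocking hit on its Box from a BP_RegularEnemy spawns an explosion, destroys the enemy and subtracts the ApplyDamage return value from health.
; At zero health it destroys itself and shows WB_Defeat.
; Tick updates its health bar widget; logic rotating the bar toward the camera is disconnected.
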(event OnComponentHit(Box)
  (params (HitComponent :type Primitive%20Component%20Object%20Reference) (OtherActor :type Actor%20Object%20Reference) (OtherComp :type Primitive%20Component%20Object%20Reference) (NormalImpulse :type Vector :default "0, 0, 0") (Hit :type Hit%20Result%20Structure%20%28by%20ref%29))
  (bind (_bblockinghit _binitialoverlap _time _distance _location _impactpoint) (Collision|BreakHitResult Hit))
  (if _bblockinghit
    (bind _asbp_regular_enemy (Utilities|Casting|CastToBP_RegularEnemy OtherActor))
    (bind _output_get (Variables|Default|SetImpactPoint _impactpoint))
    (Effects|SpawnEmitteratLocation "/Game/StarterContent/Particles/P_Explosion.P_Explosion" _output_get "0, 0, 0" "10.000000,10.000000,10.000000")
    (Audio|PlaySoundatLocation "/Game/StarterContent/Audio/Explosion01.Explosion01" _output_get "0, 0, 0" 1.0 1.0 0.0 0 0 0 0)
    (bind _returnvalue (Game|Damage|ApplyDamage self (Variables|Default|GetBaseDamage) 0 0))
    (Actor|DestroyActor _asbp_regular_enemy)
    (if (> (Variables|Default|GetCurrentHealth) 0.0)
      (bind _output_get_2 (Variables|Default|SetCurrentHealth (- (Variables|Default|GetCurrentHealth) _returnvalue)))
      (if (<= _output_get_2 0.0)
        (Actor|DestroyActor)
        (bind _returnvalue_2 (UserInterface|CreateWidget "/Game/Owned/HUD/WB_Defeat.WB_Defeat_C"))
        (bind _output_get_3 (Variables|Default|SetDefeatScreen _returnvalue_2))
        (UserInterface|Viewport|AddtoViewport _output_get_3 0)
        (Widget|SetVisibility _output_get_3 "Visible")))))

(event EventTick
  (params (DeltaSeconds :type Float%20%28single-precision%29))
  (Progress|SetPercent (Variables|/Game/Owned/HUD/WB_BaseHealthBar.WB_BaseHealthBar_C|GetHealthBar (Variables|Default|GetAs%20WB%20Base%20Health%20Bar)) (/ (Variables|Default|GetCurrentHealth) (Variables|Default|GetMaxHealth))))

(event EventBeginPlay
  (bind _aswb_base_health_bar (Utilities|Casting|CastToWB_BaseHealthBar (UserInterface|GetUserWidgetObject (Variables|Default|GetHealthBar))))
  (Variables|Default|SetAs%20WB%20Base%20Health%20Bar _aswb_base_health_bar))

(fn ConstructionScript)