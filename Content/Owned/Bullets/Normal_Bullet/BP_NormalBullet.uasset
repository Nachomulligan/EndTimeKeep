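; Bullet projectile that damages BP_RegularEnemy actors and destroys itself after a short lifetime.
; Box overlap spawns an explosion at any hit actor, then applies damage and destroys the bullet only if the enemy cast succeeds.
; AimAtTarget points velocity and rotation toward Target, but its only call here, alongside homing setup, is in unconnected logic.
; Older disabled hit-handling variants remain in the graph.
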(event OnComponentBeginOverlap(Box)
  (params (OverlappedComponent :type Primitive%20Component%20Object%20Reference) (OtherActor :type Actor%20Object%20Reference) (OtherComp :type Primitive%20Component%20Object%20Reference) (OtherBodyIndex :type Integer) (bFromSweep :type Boolean) (SweepResult :type Hit%20Result%20Structure%20%28by%20ref%29))
  (bind _hitactor (Collision|BreakHitResult SweepResult))
  (Effects|SpawnEmitteratLocation "/Game/StarterContent/Particles/P_Explosion.P_Explosion" (Transformation|GetActorLocation _hitactor))
  (Utilities|Casting|CastToBP_RegularEnemy _hitactor)
  (Game|Damage|ApplyDamage _hitactor (Variables|Default|GetDamage) 0 0)
  (Actor|DestroyActor))

(event Custom|Aim%20At%20Target
  (bind _output_get (Variables|/Script/Engine.MovementComponent|SetVelocity (Variables|Default|GetProjectileMovement) (Math|Vector|GetUnitDirection(Vector) (Transformation|GetActorLocation) (Transformation|GetActorLocation (Variables|Default|GetTarget)))))
  (Transformation|SetActorRotation (Math|Conversions|RotationFromXVector _output_get)))

(event EventBeginPlay
  (Utilities|FlowControl|Delay 3.0)
  (Actor|DestroyActor))

(fn ConstructionScript)