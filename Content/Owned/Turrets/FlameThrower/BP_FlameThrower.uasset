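; Flamethrower turret that reacts to pawn sensing by aiming at the nearest BP_RegularEnemy and firing.
; Each sighting refreshes the enemy list, then turns the Swivel with a 90-degree yaw offset, mapping inverted pitch to roll.
; A Delay paces shots, spawning BP_NormalBullet at the Arrow while any regular enemy exists.
; AC_Health depletion destroys the turret.
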(event OnSeePawn(PawnSensing)
  (params (Pawn :type Pawn%20Object%20Reference))
  (bind _outactors (Actor|GetAllActorsOfClass "/Game/Owned/Enemies/Regular_Enemy/BP_RegularEnemy.BP_RegularEnemy_C"))
  (Variables|Default|SetTarget%20List _outactors)
  (Utilities|IsValid (.ReturnValue (Actor|FindNearestActor (Transformation|GetActorLocation) (Variables|Default|GetTarget%20List)))
    (:Is%20Valid
      (CallFunction|Rotate)
      (CallFunction|Attack))))

(event OnHealthChanged(AC_Health)
  (params (NewHealth :type Float%20%28double-precision%29)))

(event OnHealthDepleted(AC_Health)
  (Actor|DestroyActor))

(event Custom|Death
  (Actor|DestroyActor))

(event Custom|Rotate
  (bind _returnvalue (Transformation|GetActorLocation))
  (bind _swivel (Variables|Default|GetSwivel))
  (bind _target_list (Variables|Default|GetTarget%20List))
  (bind _returnvalue_2 (Transformation|GetWorldLocation _swivel))
  (bind _returnvalue_3 (Actor|FindNearestActor _returnvalue _target_list))
  (bind _returnvalue_4 (Transformation|GetActorLocation _returnvalue_3))
  (bind _returnvalue_5 (+ "" _returnvalue_4))
  (bind _returnvalue_6 (Math|Rotator|FindLookatRotation _returnvalue_2 _returnvalue_5))
  (bind _returnvalue_7 (Math|Rotator|GetRotationXVector _returnvalue_6))
  (bind _returnvalue_8 (Math|Vector|RotateVector _returnvalue_7 "0.000000,-90.000000,0.000000"))
  (bind _returnvalue_9 (Math|Conversions|RotationFromXVector _returnvalue_8))
  (Transformation|SetWorldRotation (Variables|Default|GetSwivel) (Math|Rotator|MakeRotator (* (.pitch _returnvalue_9) -1.0) 0.0 (.yaw _returnvalue_9)) false false))

(event Custom|Take%20Damage
  (Game|Damage|ApplyDamage self 1e+01 0 0))

(event Custom|Attack
  (Utilities|FlowControl|Delay (Variables|Default|GetFire%20Rate))
  (bind _returnvalue (Actor|GetActorOfClass "/Game/Owned/Enemies/Regular_Enemy/BP_RegularEnemy.BP_RegularEnemy_C"))
  (Utilities|IsValid _returnvalue
    (:Is%20Valid
      (Game|SpawnActorfromClass "/Game/Owned/Bullets/Normal_Bullet/BP_NormalBullet.BP_NormalBullet_C" (Transformation|GetWorldTransform (Variables|Default|GetArrow)) "Undefined" "MultiplyWithRoot" 0 0 0))))

(fn ConstructionScript
  (|CallParentFunction))