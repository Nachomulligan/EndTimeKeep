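; BP_BaseTurret is a turret base Blueprint with a floating health bar and death handling.
; On BeginPlay it caches the WB_TurretHealthBar widget, then each Tick sets its percent from AC_HealthAllies and rotates it toward the player camera.
; TurretDeath and AC_Health depletion destroy the actor, while DamageTurret applies fixed damage to itself.
; PawnSensing and health-changed events are empty, so it contains no targeting or firing logic.
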(event OnSeePawn(PawnSensing)
  (params (Pawn :type Pawn%20Object%20Reference)))

(event OnHealthChanged(AC_Health)
  (params (NewHealth :type Float%20%28double-precision%29)))

(event OnHealthDepleted(AC_Health)
  (Actor|DestroyActor))

(event Custom|TurretDeath
  (Actor|DestroyActor))

(event Custom|DamageTurret
  (Game|Damage|ApplyDamage self 1e+01 0 0))

(event EventTick
  (params (DeltaSeconds :type Float%20%28single-precision%29))
  (bind _self self)
  (bind _healthbarturret (Variables|Default|GetHealthBarTurret))
  (bind _returnvalue (Actor|GetComponentbyClass _self "/Game/Owned/Component/AC_HealthAllies.AC_HealthAllies_C"))
  ;[1 1 1] Health Bar Config
  (Progress|SetPercent (Variables|/Game/Owned/HUD/WB_TurretHealthBar.WB_TurretHealthBar_C|GetHealthBar (Variables|Default|GetAs%20WB%20Turret%20Health%20Bar)) (/ (Variables|/Game/Owned/Component/AC_HealthAllies.AC_HealthAllies_C|GetCurrent%20Health _returnvalue) (Variables|/Game/Owned/Component/AC_HealthAllies.AC_HealthAllies_C|GetMax%20Health _returnvalue)))
  (Transformation|SetWorldRotation _healthbarturret (Math|Rotator|FindLookatRotation (Transformation|GetWorldLocation _healthbarturret) (Transformation|GetWorldLocation (Variables|/Script/Engine.Actor|GetRootComponent (Game|GetPlayerCameraManager 0)))) false false))

(event EventBeginPlay
  ;[1 1 1] Health Bar Config
  (bind _aswb_turret_health_bar (Utilities|Casting|CastToWB_TurretHealthBar (UserInterface|GetUserWidgetObject (Variables|Default|GetHealthBarTurret))))
  (Variables|Default|SetAs%20WB%20Turret%20Health%20Bar _aswb_turret_health_bar))

(fn ConstructionScript)