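; BP_MinigunShadow is the placement preview for a minigun turret, showing whether it can be built at its current spot.
; Each tick it runs a box trace around itself for WorldDynamic objects to detect an obstructed build zone.
; The Base, Swivel and Cannon meshes switch to the invalid material when blocked or when the player's Resources are below TurretPrice.
; CanBuild reflects only the obstruction check, not affordability.
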(event Custom|DetectBuildZone
  (bind _returnvalue (Transformation|GetActorLocation))
  (bind _returnvalue_2 (Transformation|GetActorLocation))
  (bind _returnvalue_3 (Class|KismetSystemLibrary|BoxTraceSingleforObjects (Math|Vector|MakeVector (.x _returnvalue) (.y _returnvalue) (+ (.z _returnvalue) 7e+01)) (Math|Vector|MakeVector (.x _returnvalue_2) (.y _returnvalue_2) (+ (.z _returnvalue_2) 7e+01)) "100.000000,250.000000,80.000000" "0, 0, 0" (Utilities|Array|MakeArray "ObjectTypeQuery2") false 0 "ForOneFrame" true "(R=0.000000,G=1.000000,B=0.000000,A=1.000000)" "(R=1.000000,G=0.000000,B=0.000000,A=1.000000)"))
  (Rendering|Material|SetMaterial (Variables|Default|GetBase) 0 (select (or _returnvalue_3 (< (Variables|/Game/FirstPerson/Blueprints/BP_FirstPersonCharacter.BP_FirstPersonCharacter_C|GetResources (stale EventBeginPlay _returnvalue)) (Variables|/Game/FirstPerson/Blueprints/BP_FirstPersonCharacter.BP_FirstPersonCharacter_C|GetTurretPrice (stale EventBeginPlay _returnvalue)))) "/Game/Owned/Turrets/Base_Turret/M_NotTurretBuildMode.M_NotTurretBuildMode" "/Game/Owned/Turrets/SingleShot_Turret/M_TurretBuildMode.M_TurretBuildMode"))
  (Variables|Default|SetCanBuild (not _returnvalue_3)))

(event EventBeginPlay
  (bind _returnvalue (Actor|GetActorOfClass "/Game/FirstPerson/Blueprints/BP_FirstPersonCharacter.BP_FirstPersonCharacter_C")))

(event EventTick
  (params (DeltaSeconds :type Float%20%28single-precision%29))
  (CallFunction|DetectBuildZone))

(fn ConstructionScript
  (|CallParentFunction))