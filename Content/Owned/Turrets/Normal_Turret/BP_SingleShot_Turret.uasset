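; Single-shot turret that aims at regular enemies it sees and fires normal bullets.
; PawnSensing turns the Swivel toward the enemy with a 90-degree correction, and a one-second Delay throttles bullet spawns from the Arrow.
; Firing only checks that some regular enemy still exists, not the sighted one.
; AC_Health destroys the turret when depleted; custom events provide self-damage, debug printing and direct destruction.
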(event OnSeePawn(PawnSensing)
  (params (Pawn :type Pawn%20Object%20Reference))
  (bind _returnvalue (Transformation|GetActorLocation Pawn))
  (bind _swivel (Variables|Default|GetSwivel))
  (bind _returnvalue_2 (Transformation|GetWorldLocation _swivel))
  (bind _returnvalue_3 (+ "" _returnvalue))
  (bind _returnvalue_4 (Math|Rotator|FindLookatRotation _returnvalue_2 _returnvalue_3))
  (bind _returnvalue_5 (Math|Rotator|GetRotationXVector _returnvalue_4))
  (bind _returnvalue_6 (Math|Vector|RotateVector _returnvalue_5 "0.000000,-90.000000,0.000000"))
  (bind _returnvalue_7 (Math|Conversions|RotationFromXVector _returnvalue_6))
  (Utilities|Casting|CastToBP_RegularEnemy Pawn)
  (Transformation|SetWorldRotation (Variables|Default|GetSwivel) (Math|Rotator|MakeRotator (* (.pitch _returnvalue_7) -1.0) 0.0 (.yaw _returnvalue_7)) false false)
  (Utilities|FlowControl|Delay 1.0)
  (bind _returnvalue_8 (Actor|GetActorOfClass "/Game/Owned/Enemies/Regular_Enemy/BP_RegularEnemy.BP_RegularEnemy_C"))
  (Utilities|IsValid _returnvalue_8
    (:Is%20Valid
      (Game|SpawnActorfromClass "/Game/Owned/Bullets/Normal_Bullet/BP_NormalBullet.BP_NormalBullet_C" (Transformation|GetWorldTransform (Variables|Default|GetArrow)) "Undefined" "MultiplyWithRoot" 0 0 0))))

(event OnHealthChanged(AC_Health)
  (params (NewHealth :type Float%20%28double-precision%29))
  (Development|PrintString (Utilities|String|Append "NewHealth" (Utilities|String|ToString(Float) NewHealth))))

(event OnHealthDepleted(AC_Health)
  (Actor|DestroyActor))

(event Custom|CustomEvent_1
  (Actor|DestroyActor))

(event Custom|CustomEvent
  (Game|Damage|ApplyDamage self 1e+01 0 0)
  (Development|PrintString "ayyyyyyy"))

(event EventBeginPlay)

(event Collision|EventActorBeginOverlap
  (params (OtherActor :type Actor%20Object%20Reference)))

(event EventTick
  (params (DeltaSeconds :type Float%20%28single-precision%29)))

(fn ConstructionScript
  (|CallParentFunction))