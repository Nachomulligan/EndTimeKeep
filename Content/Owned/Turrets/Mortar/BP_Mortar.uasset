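; BP_Mortar is a mortar turret that drops area-of-effect bullets on regular enemies and is destroyed when its health depletes.
; Pawn sensing triggers a fire-rate-delayed attack that spawns BP_AOEBullet high above an enemy, with temporary smoke at the turret.
; The nearest-enemy search only gates firing, as the attack targets whichever enemy GetActorOfClass returns.
; Cannon aiming and an older attack chain are left unwired.
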(event OnSeePawn(PawnSensing)
  (params (Pawn :type Pawn%20Object%20Reference))
  (bind _outactors (Actor|GetAllActorsOfClass "/Game/Owned/Enemies/Regular_Enemy/BP_RegularEnemy.BP_RegularEnemy_C"))
  (Variables|Default|SetTarget%20List _outactors)
  (Utilities|IsValid (.ReturnValue (Actor|FindNearestActor (Transformation|GetActorLocation) (Variables|Default|GetTarget%20List)))
    (:Is%20Valid
      (CallFunction|Attack))))

(event OnHealthChanged(AC_Health)
  (params (NewHealth :type Float%20%28double-precision%29)))

(event OnHealthDepleted(AC_Health)
  (Actor|DestroyActor))

(event Custom|Take%20Damage
  (Game|Damage|ApplyDamage self 1e+01 0 0))

(event Custom|Attack
  (Utilities|FlowControl|Delay (Variables|Default|GetFire%20Rate))
  (bind _returnvalue (Actor|GetActorOfClass "/Game/Owned/Enemies/Regular_Enemy/BP_RegularEnemy.BP_RegularEnemy_C"))
  (Utilities|IsValid _returnvalue
    (:Is%20Valid
      (Game|SpawnActorfromClass "/Game/Owned/Bullets/BP_AOEBullet.BP_AOEBullet_C" (Math|Transform|MakeTransform (Math|Vector|MakeVector (.x (Transformation|GetActorLocation _returnvalue)) (.y (Transformation|GetActorLocation _returnvalue)) (+ (.z (Transformation|GetActorLocation _returnvalue)) 4e+03)) "0, 0, 0" "1.000000,1.000000,1.000000") "Undefined" "MultiplyWithRoot" 0 0)
      (bind _returnvalue_2 (Effects|SpawnEmitteratLocation "/Game/StarterContent/Particles/P_Smoke.P_Smoke" (Transformation|GetWorldLocation (Variables|Default|GetScene))))
      (Utilities|FlowControl|Delay 2.0)
      (Components|DestroyComponent _returnvalue_2))))

(fn ConstructionScript
  (|CallParentFunction))