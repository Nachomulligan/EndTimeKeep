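; BP_WaveSpawner is an interactable that spawns a timed wave of BP_RegularEnemy actors when E is pressed.
; Any overlap with its Box enables input from player 0, and ending overlap calls DisableInput on that player controller.
; Spawn counts down from WaveAmount in a delayed loop, waiting SpawnCooldown before placing each enemy at a random reachable point around the Scene component.
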(event OnComponentBeginOverlap(Box)
  (params (OverlappedComponent :type Primitive%20Component%20Object%20Reference) (OtherActor :type Actor%20Object%20Reference) (OtherComp :type Primitive%20Component%20Object%20Reference) (OtherBodyIndex :type Integer) (bFromSweep :type Boolean) (SweepResult :type Hit%20Result%20Structure%20%28by%20ref%29))
  (Input|EnableInput (Game|GetPlayerController 0)))

(event OnComponentEndOverlap(Box)
  (params (OverlappedComponent :type Primitive%20Component%20Object%20Reference) (OtherActor :type Actor%20Object%20Reference) (OtherComp :type Primitive%20Component%20Object%20Reference) (OtherBodyIndex :type Integer))
  (Input|DisableInput (Game|GetPlayerController 0) 0))

(event Custom|Spawn
  (bind _output_get (Variables|Default|SetCurrentWave (Variables|Default|GetWaveAmount)))
  (if (> _output_get 0) :!label _label
    (Utilities|FlowControl|Delay (Variables|Default|GetSpawnCooldown))
    (Game|SpawnActorfromClass "/Game/Owned/Enemies/Regular_Enemy/BP_RegularEnemy.BP_RegularEnemy_C" (Math|Transform|MakeTransform (.RandomLocation (AI|Navigation|GetRandomReachablePointinRadius (Transformation|GetWorldLocation (Variables|Default|GetScene)) 1e+03 0 0)) "0, 0, 0" "1.000000,1.000000,1.000000") "Undefined" "MultiplyWithRoot" 0 0)
    (Math|Integer|DecrementInt (Variables|Default|GetCurrentWave)
      (:%20%20
        (goto _label)))))

(event Input|KeyboardEvents|E
  (params (Key :type Key%20Structure :default "None"))
  (:Pressed
    (CallFunction|Spawn)))

(fn ConstructionScript)