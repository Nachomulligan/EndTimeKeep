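; BP_LoadScene is an interactable that loads another level when the player presses E while inside its trigger box.
; Box overlap begin enables input from the first player controller, and overlap end calls DisableInput on that controller without filtering the overlapping actor.
; The E press confirms the player is BP_FirstPersonCharacter, shows a WB_Fade widget, plays its fade animation, then opens the referenced Level after a one-second delay.
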(event OnComponentBeginOverlap(Box)
  (params (OverlappedComponent :type Primitive%20Component%20Object%20Reference) (OtherActor :type Actor%20Object%20Reference) (OtherComp :type Primitive%20Component%20Object%20Reference) (OtherBodyIndex :type Integer) (bFromSweep :type Boolean) (SweepResult :type Hit%20Result%20Structure%20%28by%20ref%29))
  (Input|EnableInput (Game|GetPlayerController 0)))

(event OnComponentEndOverlap(Box)
  (params (OverlappedComponent :type Primitive%20Component%20Object%20Reference) (OtherActor :type Actor%20Object%20Reference) (OtherComp :type Primitive%20Component%20Object%20Reference) (OtherBodyIndex :type Integer))
  (Input|DisableInput (Game|GetPlayerController 0) 0))

(event Input|KeyboardEvents|E
  (params (Key :type Key%20Structure :default "None"))
  (:Pressed
    (Utilities|Casting|CastToBP_FirstPersonCharacter (Game|GetPlayerCharacter 0))
    (bind _returnvalue (Game|ConstructObjectfromClass "/Game/Owned/HUD/WB_Fade.WB_Fade_C"))
    (UserInterface|Viewport|AddtoViewport _returnvalue 0)
    (Default|FadeAnimation _returnvalue)
    (Utilities|FlowControl|Delay 1.0)
    (Game|OpenLevel(byObjectReference) (Variables|Default|GetLevel))))

(fn ConstructionScript)