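; BP_InteractShow is a trigger actor that toggles the player's interaction widget based on proximity.
; On BeginPlay it caches player 0's character and casts it to BP_FirstPersonCharacter.
; Its Box collision component calls ShowInteractionWidget on that character when the player begins overlapping and HideInteractionWidget when the overlap ends, ignoring other actors.
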(event OnComponentBeginOverlap(Box)
  (params (OverlappedComponent :type Primitive%20Component%20Object%20Reference) (OtherActor :type Actor%20Object%20Reference) (OtherComp :type Primitive%20Component%20Object%20Reference) (OtherBodyIndex :type Integer) (bFromSweep :type Boolean) (SweepResult :type Hit%20Result%20Structure%20%28by%20ref%29))
  (if (== OtherActor (Variables|Default|GetPlayerCharacter))
    (Default|ShowInteractionWidget (Variables|Default|GetAs%20BP%20First%20Person%20Character))))

(event OnComponentEndOverlap(Box)
  (params (OverlappedComponent :type Primitive%20Component%20Object%20Reference) (OtherActor :type Actor%20Object%20Reference) (OtherComp :type Primitive%20Component%20Object%20Reference) (OtherBodyIndex :type Integer))
  (if (== (Variables|Default|GetPlayerCharacter) OtherActor)
    (Default|HideInteractionWidget (Variables|Default|GetAs%20BP%20First%20Person%20Character))))

(event EventBeginPlay
  (bind _output_get (Variables|Default|SetPlayerCharacter (Game|GetPlayerCharacter 0)))
  (bind _asbp_first_person_character (Utilities|Casting|CastToBP_FirstPersonCharacter _output_get))
  (Variables|Default|SetAs%20BP%20First%20Person%20Character _asbp_first_person_character))

(fn ConstructionScript)