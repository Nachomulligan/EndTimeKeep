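; BP_Radio is an interactable radio that the player toggles on and off.
; Each Interact event runs through a FlipFlop and plays a switch sound at the radio mesh's location.
; Switching on starts the RadioStation audio from the beginning after a one-second delay, while switching off stops it immediately.
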(event EventInteract
  (Utilities|FlowControl|FlipFlop
    (:A
      (Audio|PlaySoundatLocation "/Game/Assets/Sounds/switchSound.switchSound" (Transformation|GetWorldLocation (Variables|Default|GetSM_Radio)) "0, 0, 0" 1.0 1.0 0.0 "/Game/Assets/Sounds/Attenuation/SA_All.SA_All" 0 0 0)
      (Utilities|FlowControl|Delay 1.0)
      (Audio|Components|Audio|Play (Variables|Default|GetRadioStation) 0.0))
    (:B
      (Audio|PlaySoundatLocation "/Game/Assets/Sounds/switchSound.switchSound" (Transformation|GetWorldLocation (Variables|Default|GetSM_Radio)) "0, 0, 0" 1.0 1.0 0.0 "/Game/Assets/Sounds/Attenuation/SA_All.SA_All" 0 0 0)
      (Audio|Components|Audio|Stop (Variables|Default|GetRadioStation)))))

(fn ConstructionScript)