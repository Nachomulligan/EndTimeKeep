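; Interactable button that spawns a series of regular enemies around its location when used.
; Interact plays a button sound, then runs a delayed loop that counts down from the wave amount, spawning one BP_RegularEnemy after each cooldown.
; Each spawn location is a random reachable navigation point within a fixed radius of the Scene component.
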(event EventInteract
  (Audio|PlaySound2D "/Game/Assets/Sounds/Button_Gameplay.Button_Gameplay" 1.0 1.0 0.0 0 0)
  (bind _output_get (Variables|Default|SetCurrentWave (Variables|Default|GetWaveAmount)))
  (if (> _output_get 0) :!label _label
    (Utilities|FlowControl|Delay (Variables|Default|GetSpawnCooldown))
    (Game|SpawnActorfromClass "/Game/FirstPerson/Blueprints/EnemyBlueprints/Regular_Enemy/BP_RegularEnemy.BP_RegularEnemy_C" (Math|Transform|MakeTransform (.RandomLocation (AI|Navigation|GetRandomReachablePointinRadius (Transformation|GetWorldLocation (Variables|Default|GetScene)) 1e+03 0 0)) "0, 0, 0" "1.000000,1.000000,1.000000") "Undefined" "MultiplyWithRoot" 0 0)
    (Math|Integer|DecrementInt (Variables|Default|GetCurrentWave)
      (:%20%20
        (goto _label)))))

(fn ConstructionScript)