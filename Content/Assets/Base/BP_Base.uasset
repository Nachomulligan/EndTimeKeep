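; BP_Base is the base that regular enemies damage on impact, opening the lose screen when its health runs out.
; A blocking Box hit from BP_RegularEnemy spawns an explosion with sound, destroys the enemy and subtracts the ApplyDamage result from CurrentHealth.
; Tick pushes the health ratio to the health bar widget, which stays hidden for a fixed delay after BeginPlay.
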(event OnComponentHit(Box)
  (params (HitComponent :type Primitive%20Component%20Object%20Reference) (OtherActor :type Actor%20Object%20Reference) (OtherComp :type Primitive%20Component%20Object%20Reference) (NormalImpulse :type Vector :default "0, 0, 0") (Hit :type Hit%20Result%20Structure%20%28by%20ref%29))
  (bind (_bblockinghit _binitialoverlap _time _distance _location _impactpoint) (Collision|BreakHitResult Hit))
  ;[1 1 1] Base Hit by Enemy and Death
  (Variables|Default|SetOther%20Actor OtherActor)
  (if _bblockinghit
    (Variables|Default|SetImpactPoint _impactpoint)
    (bind _asbp_regular_enemy (Utilities|Casting|CastToBP_RegularEnemy (Variables|Default|GetOther%20Actor)))
    (Variables|Default|SetAs%20BP%20Regular%20Enemy _asbp_regular_enemy)
    (Effects|SpawnEmitteratLocation "/Game/StarterContent/Particles/P_Explosion.P_Explosion" (Variables|Default|GetImpactPoint) "0, 0, 0" "10.000000,10.000000,10.000000")
    (Audio|PlaySoundatLocation "/Game/StarterContent/Audio/Explosion01.Explosion01" (Variables|Default|GetImpactPoint) "0, 0, 0" 1.0 1.0 0.0 0 0 0 0)
    (bind _returnvalue (Game|Damage|ApplyDamage self (Variables|Default|GetBaseDamage) 0 0))
    (Actor|DestroyActor (Variables|Default|GetAs%20BP%20Regular%20Enemy))
    (if (> (Variables|Default|GetCurrentHealth) 0.0)
      (bind _output_get (Variables|Default|SetCurrentHealth (- (Variables|Default|GetCurrentHealth) _returnvalue)))
      (if (<= _output_get 0.0)
        (CallFunction|Death)))))

(event Custom|Death
  ;[1 1 1] Death
  (Actor|DestroyActor)
  (Game|OpenLevel(byObjectReference) "/Game/FirstPerson/Maps/LoseMenuScreen.LoseMenuScreen"))

(event Custom|ShowHealthBarBase
  ;[1 1 1] Show/Hide Health Bar
  (Development|SetHiddeninGame (Variables|Default|GetHealthBar) false false))

(event Custom|HideHealthBarBase
  ;[1 1 1] Show/Hide Health Bar
  (Development|SetHiddeninGame (Variables|Default|GetHealthBar) true false))

(event EventTick
  (params (DeltaSeconds :type Float%20%28single-precision%29))
  ;[1 1 1] Base Health
  (Progress|SetPercent (Variables|/Game/Assets/HUD/WB_BaseHealthBar.WB_BaseHealthBar_C|GetHealthBar (Variables|Default|GetAs%20WB%20Base%20Health%20Bar)) (/ (Variables|Default|GetCurrentHealth) (Variables|Default|GetMaxHealth))))

(event EventBeginPlay
  ;[1 1 1] Base Health
  (bind _aswb_base_health_bar (Utilities|Casting|CastToWB_BaseHealthBar (UserInterface|GetUserWidgetObject (Variables|Default|GetHealthBar))))
  (Variables|Default|SetAs%20WB%20Base%20Health%20Bar _aswb_base_health_bar)
  (CallFunction|HideHealthBarBase)
  (Utilities|FlowControl|Delay 14.1)
  (CallFunction|ShowHealthBarBase))

(fn ConstructionScript)