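; BP_MortarShadow is the placement preview for a mortar turret, showing whether the player can build at its location.
; Each tick, a debug-drawn, zero-length box trace just above the actor checks one object type for obstructions.
; Base and Cannon switch to the blocked material on a hit or when the first-person character's resources are below the turret price.
; CanBuild reflects only the trace result, not affordability.
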(event Custom|DetectBuildZone
  (bind _returnvalue (Transformation|GetActorLocation))
  (bind _returnvalue_2 (Transformation|GetActorLocation))
  ;[1 1 1] Where can Player build
  (bind _returnvalue_3 (Class|KismetSystemLibrary|BoxTraceSingleforObjects (Math|Vector|MakeVector (.x _returnvalue) (.y _returnvalue) (+ (.z _returnvalue) 1e+02)) (Math|Vector|MakeVector (.x _returnvalue_2) (.y _returnvalue_2) (+ (.z _returnvalue_2) 1e+02)) "100.000000,250.000000,110.000000" "0, 0, 0" (Utilities|Array|MakeArray "ObjectTypeQuery10") false 0 "ForOneFrame" true "(R=0.000000,G=1.000000,B=0.000000,A=1.000000)" "(R=1.000000,G=0.000000,B=0.000000,A=1.000000)"))
  ;[1 1 1] Paints the shadow with green or red
  (Rendering|Material|SetMaterial (Variables|Default|GetBase) 0 (select (or _returnvalue_3 (< (Variables|/Game/FirstPerson/Blueprints/BP_FirstPersonCharacter.BP_FirstPersonCharacter_C|GetResources (stale EventBeginPlay _returnvalue)) (Variables|/Game/FirstPerson/Blueprints/BP_FirstPersonCharacter.BP_FirstPersonCharacter_C|GetTurretPrice (stale EventBeginPlay _returnvalue)))) "/Game/Assets/Turrets/Base_Turret/M_NotTurretBuildMode.M_NotTurretBuildMode" "/Game/Assets/Turrets/SingleShot_Turret/M_TurretBuildMode.M_TurretBuildMode"))
  ;[1 1 1] Allows BuildMode
  (Variables|Default|SetCanBuild (not _returnvalue_3)))

(event EventBeginPlay
  ;[1 1 1] Player has resources
  (bind _returnvalue (Actor|GetActorOfClass "/Game/FirstPerson/Blueprints/BP_FirstPersonCharacter.BP_FirstPersonCharacter_C")))

(event EventTick
  (params (DeltaSeconds :type Float%20%28single-precision%29))
  ;[1 1 1] Where can Player build
  (CallFunction|DetectBuildZone))

(fn ConstructionScript
  (|CallParentFunction))