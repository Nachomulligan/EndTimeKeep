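; Mortar turret that drops BP_AOEBullet shells from high above enemies and dies when its health depletes.
; Sighting an "Enemy"-tagged pawn triggers a FireRate-delayed attack above the first BP_RegularEnemy found; the nearest-actor search only gates firing.
; Each shot plays sound and a temporary explosion effect at the Scene component.
; TakeDamage self-applies fixed damage, AC_Health depletion destroys the turret, and older firing and aiming logic sits unconnected.
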(event OnSeePawn(PawnSensing)
  (params (Pawn :type Pawn%20Object%20Reference))
  (if (Actor|ActorHasTag Pawn "Enemy")
    (bind _outactors (Actor|GetAllActorsOfClass "/Game/FirstPerson/Blueprints/EnemyBlueprints/Regular_Enemy/BP_RegularEnemy.BP_RegularEnemy_C"))
    (Variables|Default|SetTarget%20List _outactors)
    (Utilities|IsValid (.ReturnValue (Actor|FindNearestActor (Transformation|GetActorLocation) (Variables|Default|GetTarget%20List)))
      (:Is%20Valid
        (CallFunction|Attack)))))

(event OnHealthChanged(AC_Health)
  (params (NewHealth :type Float%20%28double-precision%29)))

(event OnHealthDepleted(AC_Health)
  (Audio|PlaySoundatLocation "/Game/Assets/Sounds/Turret_death.Turret_death" (Transformation|GetActorLocation) "0, 0, 0" 1.0 1.0 0.0 "/Game/Assets/Sounds/Attenuation/SA_All.SA_All" 0 0 0)
  (Utilities|FlowControl|Delay 0.5)
  (Actor|DestroyActor))

(event Custom|PlayVFX
  (bind _returnvalue (Effects|SpawnEmitteratLocation "/Game/StarterContent/Particles/P_Explosion.P_Explosion" (Transformation|GetWorldLocation (Variables|Default|GetScene)))))

(event Custom|PlaySFX
  (Audio|PlaySoundatLocation "/Game/Assets/Sounds/Mortar_shot_sound.Mortar_shot_sound" (Transformation|GetActorLocation) "0, 0, 0" 1.0 1.0 0.0 "/Game/Assets/Sounds/Attenuation/SA_All.SA_All" 0 0 0))

(event Custom|Take%20Damage
  (Game|Damage|ApplyDamage self 1e+01 0 0))

(event Custom|Attack
  (Utilities|FlowControl|Delay (Variables|Default|GetFire%20Rate))
  (bind _returnvalue (Actor|GetActorOfClass "/Game/FirstPerson/Blueprints/EnemyBlueprints/Regular_Enemy/BP_RegularEnemy.BP_RegularEnemy_C"))
  (Utilities|IsValid _returnvalue
    (:Is%20Valid
      (Game|SpawnActorfromClass "/Game/Assets/Bullets/BP_AOEBullet.BP_AOEBullet_C" (Math|Transform|MakeTransform (Math|Vector|MakeVector (.x (Transformation|GetActorLocation _returnvalue)) (.y (Transformation|GetActorLocation _returnvalue)) (+ (.z (Transformation|GetActorLocation _returnvalue)) 4e+03)) "0, 0, 0" "1.000000,1.000000,1.000000") "Undefined" "MultiplyWithRoot" 0 0)
      (CallFunction|PlayVFX)
      (CallFunction|PlaySFX)
      (Utilities|FlowControl|Delay 2.0)
      (Components|DestroyComponent (stale Custom|PlayVFX _returnvalue)))))

(fn ConstructionScript
  (|CallParentFunction))