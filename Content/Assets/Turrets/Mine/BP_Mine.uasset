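; BP_Mine is an explosive mine, filed with the turret assets, that detonates on a blocking hit to its Mine component.
; The hit spawns a scaled-up explosion effect and sound at the impact point, then the mine destroys itself.
; It then applies full, non-falloff radial damage within the explosion radius, ignoring actors tagged "Ally" and using a custom trace channel for damage blocking.
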(event OnComponentHit(Mine)
  (params (HitComponent :type Primitive%20Component%20Object%20Reference) (OtherActor :type Actor%20Object%20Reference) (OtherComp :type Primitive%20Component%20Object%20Reference) (NormalImpulse :type Vector :default "0, 0, 0") (Hit :type Hit%20Result%20Structure%20%28by%20ref%29))
  (bind (_bblockinghit _binitialoverlap _time _distance _location _impactpoint) (Collision|BreakHitResult Hit))
  (if _bblockinghit
    (bind _output_get (Variables|Default|SetImpact%20Point _impactpoint))
    (Effects|SpawnEmitteratLocation "/Game/StarterContent/Particles/P_Explosion.P_Explosion" _output_get "0, 0, 0" "10.000000,10.000000,10.000000")
    (Audio|PlaySoundatLocation "/Game/StarterContent/Audio/Explosion01.Explosion01" _output_get "0, 0, 0" 1.0 1.0 0.0 0 0 0 0)
    (bind _outactors (Actor|GetAllActorswithTag "Ally"))
    (Actor|DestroyActor)
    (Game|Damage|ApplyRadialDamage (Variables|Default|GetBase%20Damage) (Variables|Default|GetImpact%20Point) (Variables|Default|GetExplosionRadius) 0 _outactors 0 0 true "ECC_GameTraceChannel2")))

(fn ConstructionScript)